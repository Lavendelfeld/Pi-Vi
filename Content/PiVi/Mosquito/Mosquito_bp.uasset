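; Mosquito enemy for the 2D side-scroller that restarts the current level when its box overlaps the player character, destroying the character first.
; On BeginPlay a timeline lerps it from its spawn location to an offset end point, and a Paper flipbook component is added.
; The FunctionLBM event, triggered from outside this graph, plays a sound and destroys the mosquito.
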(event `self.Box.OnComponentBeginOverlap`
  (params (OverlappedComponent :type "PrimitiveComponent Object Reference") (OtherActor :type "Actor Object Reference") (OtherComp :type "PrimitiveComponent Object Reference") (OtherBodyIndex :type Integer) (bFromSweep :type Boolean) (SweepResult :type "HitResult Structure (by ref)"))
  (bind _as2dside_scroller_character (cast `/Game/PiVi/PiViCharacter/2DSideScrollerCharacter` OtherActor))
  (`self.K2_DestroyActor` _as2dside_scroller_character)
  (bind _returnvalue (`GameplayStatics.GetCurrentLevelName` true))
  (`GameplayStatics.OpenLevel` (`KismetStringLibrary.Conv_StringToName` _returnvalue)))

(event `/Game/PiVi/Bad_plants/LMB_int.Function_LBM`
  (`|ExecutionSequence`
    (:`then_0`
      (`GameplayStatics.PlaySound2D` "/Game/PiVi/sound/lmb.lmb" 1.0 1.0 0.0 null null))
    (:`then_1`
      (`self.K2_DestroyActor`))))

(event `self.ReceiveBeginPlay`
  (bind _returnvalue (`self.K2_GetActorLocation`))
  (`|ExecutionSequence`
    (:`then_0`
      (set `self.startlocation` _returnvalue)
      (set `self.endlocation` (+ _returnvalue (`self.endpoin`)))
      (bind (_direction _newtrack_0) (`Timeline|Timeline_0`)
        (:`Update`
          (`self.K2_SetActorLocation` (`KismetMathLibrary.VLerp` (`self.startlocation`) (`self.endlocation`) _newtrack_0)))))
    (:`then_1`
      (`AddComponent|NODE_AddPaperFlipbookComponent-0`))))

(fn `UserConstructionScript`)