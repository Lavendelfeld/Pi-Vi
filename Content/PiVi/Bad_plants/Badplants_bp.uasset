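; Hostile plant for a 2D side-scroller that can either be destroyed by the player or kill them.
; Player overlap with Box destroys the plant, while overlap with Box1 destroys the character and reopens the current level by name.
; A separate FunctionLBM event also destroys the plant, and BeginPlay adds a Paper2D flipbook component at runtime.
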(event `self.ReceiveBeginPlay`
  (`AddComponent|NODE_AddPaperFlipbookComponent-0`))

(event `self.Box.OnComponentBeginOverlap`
  (params (OverlappedComponent :type "PrimitiveComponent Object Reference") (OtherActor :type "Actor Object Reference") (OtherComp :type "PrimitiveComponent Object Reference") (OtherBodyIndex :type Integer) (bFromSweep :type Boolean) (SweepResult :type "HitResult Structure (by ref)"))
  (cast `/Game/PiVi/PiViCharacter/2DSideScrollerCharacter` OtherActor)
  (`self.K2_DestroyActor`))

(event `self.Box1.OnComponentBeginOverlap`
  (params (OverlappedComponent :type "PrimitiveComponent Object Reference") (OtherActor :type "Actor Object Reference") (OtherComp :type "PrimitiveComponent Object Reference") (OtherBodyIndex :type Integer) (bFromSweep :type Boolean) (SweepResult :type "HitResult Structure (by ref)"))
  (bind _as2dside_scroller_character (cast `/Game/PiVi/PiViCharacter/2DSideScrollerCharacter` OtherActor))
  (`self.K2_DestroyActor` _as2dside_scroller_character)
  (bind _returnvalue (`GameplayStatics.GetCurrentLevelName` true))
  (`GameplayStatics.OpenLevel` (`KismetStringLibrary.Conv_StringToName` _returnvalue)))

(event `/Game/PiVi/Bad_plants/LMB_int.Function_LBM`
  (`self.K2_DestroyActor`))

(fn `UserConstructionScript`)